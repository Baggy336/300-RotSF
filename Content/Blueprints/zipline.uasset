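; Zipline actor that the player interacts with to ride from the Cable to the Dismount point.
; On interaction it takes possession via BetterPlayerController and destroys the player character rather than moving it.
; A timeline, rate-scaled by AverageSpeed over distance, lerps the Camera just below the line, facing the Dismount.
; When the timeline finishes, it spawns a new PlayerCharacter at that position and yaw and possesses it.
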(event `/Game/Blueprints/Interface/IPlayerCanLookAtAndInteractWith.PlayerWantsToInteract`
  (params (PlayerCharacter :type "/Game/Blueprints/PlayerAndGame/PlayerCharacter Object Reference"))
  (bind _returnvalue (`SceneComponent.K2_GetComponentLocation` (`self.Cable`)))
  (bind _returnvalue_2 (`SceneComponent.K2_GetComponentLocation` (`self.dismount`)))
  (bind _returnvalue_3 (`KismetMathLibrary.FindLookAtRotation` _returnvalue _returnvalue_2))
  (bind _asbetter_player_controller (cast `/Game/Blueprints/PlayerAndGame/BetterPlayerController` (`GameplayStatics.GetPlayerController` 0)))
  (`/Game/Blueprints/PlayerAndGame/BetterPlayerController.PossessWithBlend` _asbetter_player_controller self 0.0)
  (`self.K2_DestroyActor` PlayerCharacter)
  (`TimelineComponent.SetPlayRate` (`self.cameraMovin`) (/ (`self.averageSpeed`) (`KismetMathLibrary.VSize` (- _returnvalue _returnvalue_2))))
  (bind (_direction _percent) (`Timeline|cameraMovin` :!via `PlayFromStart` :!label _label)
    (:`Update`
      (bind _returnvalue_4 (+ (`KismetMathLibrary.VLerp` _returnvalue _returnvalue_2 _percent) (0.0 0.0 -100.0)))
      (`SceneComponent.K2_SetWorldLocationAndRotation` (`self.Camera`) _returnvalue_4 _returnvalue_3 false false))
    (:`Finished`
      (bind _returnvalue_5 (`|SpawnActorFromClass` "/Game/Blueprints/PlayerAndGame/PlayerCharacter.PlayerCharacter_C" (`KismetMathLibrary.MakeTransform` _returnvalue_4 (`KismetMathLibrary.MakeRotator` 0.0 0.0 (.yaw _returnvalue_3))) "Undefined" "OverrideRootScale" null null))
      (bind _asbetter_player_controller_2 (cast `/Game/Blueprints/PlayerAndGame/BetterPlayerController` (`GameplayStatics.GetPlayerController` 0)))
      (`/Game/Blueprints/PlayerAndGame/BetterPlayerController.PossessWithBlend` _asbetter_player_controller_2 _returnvalue_5 0.0))))

(event `self.ReceiveBeginPlay`
  (goto _label :!via `SetNewTime`))

(fn `UserConstructionScript`)