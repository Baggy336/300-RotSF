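; An NPC that shows a multi-line dialogue box when the player interacts and spawns a configurable actor, presumably a key, after the first conversation.
; Interaction creates the widget, binds its next and close events to step through a clamped text array, and locks movement with UI-only input.
; Closing restores game input and spawns the class at a marker component once.
; A door-toggle branch exists but is unconnected.
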(event `/Game/Blueprints/Interface/IPlayerCanLookAtAndInteractWith.PlayerWantsToInteract`
  (params (PlayerCharacter :type "/Game/Blueprints/PlayerAndGame/PlayerCharacter Object Reference"))
  (bind _returnvalue (`GameplayStatics.GetPlayerController` 0))
  (set `self.arrayIndex` 0)
  (bind _returnvalue_2 (`|CreateWidget` "/Game/Blueprints/GUIs/dialougeBox.dialougeBox_C"))
  (bind _output_get (set `self.widget` _returnvalue_2))
  (`/Game/Blueprints/GUIs/dialougeBox.updatetext` _output_get (`|GetArrayItem` (`self.textCharacterSays`) (`self.arrayIndex`)))
  (add `/Game/Blueprints/GUIs/dialougeBox.closeBox` _output_get (delegate `closeDialouge`))
  (add `/Game/Blueprints/GUIs/dialougeBox.goToNextText` (`self.widget`) (delegate `goToNextText`))
  (`UserWidget.AddToPlayerScreen` _returnvalue_2 0)
  (`PlayerController.SetCinematicMode` _returnvalue true true false true true)
  (`WidgetBlueprintLibrary.SetInputMode_UIOnlyEx` _returnvalue null)
  (set `PlayerController.bShowMouseCursor` true _returnvalue))

(event `goToNextText`
  (set `self.arrayIndex` (`KismetMathLibrary.Clamp` (+ (`self.arrayIndex`) 1) 0 (- (`KismetArrayLibrary.Array_Length` (`self.textCharacterSays`)) 1)))
  (`/Game/Blueprints/GUIs/dialougeBox.updatetext` (`self.widget`) (`|GetArrayItem` (`self.textCharacterSays`) (`self.arrayIndex`))))

(event `closeDialouge`
  (bind _returnvalue (`GameplayStatics.GetPlayerController` 0))
  (bind _widget (`self.widget`))
  (bind _whattospawn (`self.whatToSpawn`))
  (`Widget.RemoveFromParent` _widget)
  (clear `/Game/Blueprints/GUIs/dialougeBox.closeBox` _widget)
  (`PlayerController.SetCinematicMode` _returnvalue false true true true true)
  (`WidgetBlueprintLibrary.SetInputMode_GameOnly` _returnvalue)
  (set `PlayerController.bShowMouseCursor` false _returnvalue)
  (if (not (`self.hasKeySpawned`))
    (set `self.hasKeySpawned` true)
    (if (`KismetSystemLibrary.IsValidClass` _whattospawn)
      (`|SpawnActorFromClass` _whattospawn (`KismetMathLibrary.MakeTransform` (`SceneComponent.K2_GetComponentLocation` (`self.spawnObject`))) "Undefined" "OverrideRootScale" null null))))

(fn `UserConstructionScript`)