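; Keyhole Blueprint that unlocks when given a matching key, then triggers the objects it controls.
; Fix accepts a held PickupableObject that opens doors and shares its KeyCode, clears IsLocked, reveals the hidden key mesh and reports success.
; A timeline slides and rotates that mesh relative to its starting transform.
; When the animation finishes, each controlled object receives a ToggleMessage reflecting the unlocked state.
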(event `self.ReceiveBeginPlay`
  (bind _mesh___key (`self.Mesh - Key`))
  (bind (_returnvalue_location _returnvalue_rotation) (`KismetMathLibrary.BreakTransform` (`SceneComponent.GetRelativeTransform` _mesh___key)))
  (`SceneComponent.SetVisibility` _mesh___key false false)
  (set `self.Key Start Location` _returnvalue_location)
  (set `self.Key Start Rotation` _returnvalue_rotation)
  (set `self.Direction to Move Key` (`KismetMathLibrary.InverseTransformDirection` (`SceneComponent.K2_GetComponentToWorld` _mesh___key) (`SceneComponent.GetForwardVector` _mesh___key)))
  (bind (_direction _local_x_pos _local_y_rotate) (`Timeline|Timeline_0` :!via `SetNewTime`)
    (:`Update`
      (`SceneComponent.K2_SetRelativeLocationAndRotation` (`self.Mesh - Key`) (+ (* (`self.Direction to Move Key`) _local_x_pos) (`self.Key Start Location`)) (`KismetMathLibrary.ComposeRotators` (`KismetMathLibrary.MakeRotator` 0.0 _local_y_rotate) (`self.Key Start Rotation`)) false true))
    (:`Finished`
      (`self.UpdateControlledObjects`))))

(fn `Fix`
  (params (`Currently held item` :type "Actor Object Reference"))
  (returns (`Is It Fixed?` :type Boolean))
  (bind _aspickupable_object (cast `/Game/Blueprints/PickupableObject` `Currently held item`)
    (:`then`
      (if (`/Game/Blueprints/PickupableObject.Opens doors` _aspickupable_object)
        (if (`self.IsLocked`)
          (if (== (`/Game/Blueprints/PickupableObject.Key code` _aspickupable_object) (`self.Key code`))
            (set `self.IsLocked` false)
            (`SceneComponent.SetVisibility` (`self.Mesh - Key`) true false)
            (`TimelineComponent.Play` (`self.Timeline_0`))
            (return true)
            (else
              _)))))
    (:`CastFailed`
      _))
  (return false))

(fn `UpdateControlledObjects`
  (for _array_element (`self.ControlledObjects`)
    (message `/Game/Blueprints/Interface/ITriggerOrToggle.Toggle` _array_element (not (`self.IsLocked`)))))

(fn `UserConstructionScript`)